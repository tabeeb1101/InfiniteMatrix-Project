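; BP_Controller is a controller Blueprint that owns the main HUD and handles click-to-fire input.
; On BeginPlay it creates a WB_Main widget, stores it and adds it to the viewport.
; UpdateScore and UpdateHealth events forward score and health values to that widget's score display and health bar.
; A MouseClick press spawns a BP_Projectile at the player pawn's location, with no rotation supplied.
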(event `UpdateScore`
  (params (Score :type "Float (double-precision)"))
  (`/Game/InfiniteMatrix/UI/WB_Main.SetScore` (`self.WB_Main`) Score))

(event `UpdateHealth`
  (params (CurrentHealth :type "Float (double-precision)") (MaxHealth :type "Float (double-precision)"))
  (`/Game/InfiniteMatrix/UI/WB_Main.SetHealthBarInfo` (`self.WB_Main`) CurrentHealth MaxHealth))

(event `self.ReceiveBeginPlay`
  (bind _returnvalue (`|CreateWidget` "/Game/InfiniteMatrix/UI/WB_Main.WB_Main_C"))
  (bind _output_get (set `self.WB_Main` _returnvalue))
  (`UserWidget.AddToViewport` _output_get 0))

(event `InputAction|MouseClick`
  (params (Key :type "Key Structure"))
  (:`Pressed`
    (`|SpawnActorFromClass` "/Game/InfiniteMatrix/Blueprints/BP_Projectile.BP_Projectile_C" (`KismetMathLibrary.MakeTransform` (`self.K2_GetActorLocation` (`GameplayStatics.GetPlayerPawn` 0))) "Undefined" "MultiplyWithRoot" null null)))

(fn `UserConstructionScript`)